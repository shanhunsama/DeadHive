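; Zombie enemy character that chases the first player and attacks in melee, spawning with a random mesh, animation set and run or sprint speed.
; Looping timers refresh AI movement and trace ahead to trigger random attack montages.
; HitDamageCheck sweeps between mesh sockets to deal damage, limited by a resettable DoOnce.
; Damage plays random hit reactions until death, which ragdolls the body, lowers render cost, requests a spawner respawn and destroys it later.
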(event `self.ReceiveBeginPlay`
  (bind _aszombie_anim (cast `/Game/Blueprints/Zombie/Zombie_Anim` (`SkeletalMeshComponent.GetAnimInstance` (`self.Mesh`))))
  (set `self.As Zombie Anim` _aszombie_anim)
  (`KismetSystemLibrary.K2_SetTimer` null "ChasePlayer" 1.0 true)
  (`self.Init velocity and anim`)
  (`self.RandomZombie`)
  (`KismetSystemLibrary.K2_SetTimer` null "attackRangeCheck" 1.0 true))

(event `ChasePlayer`
  (bind _returnvalue (`GameplayStatics.GetPlayerPawn` 0))
  (`|AIMoveTo` self (0.0 0.0 0.0) _returnvalue 100.0
    (:`then`
      (`AIController.K2_SetFocus` (`AIBlueprintHelperLibrary.GetAIController` self) _returnvalue))))

(event `self.ReceiveAnyDamage`
  (params (Damage :type "Float (single-precision)") (DamageType :type "DamageType Object Reference") (InstigatedBy :type "Controller Object Reference") (DamageCauser :type "Actor Object Reference"))
  (bind _mesh (`self.Mesh`))
  (bind _mesh_2 (`self.Mesh`))
  (bind _output_get (set `self.CurrBlood` (- (`self.CurrBlood`) Damage)))
  (if (<= _output_get 0.0)
    (`/Engine/EditorBlueprintResources/StandardMacros.DoOnce` false
      (:`Completed`
        (`PrimitiveComponent.SetCollisionEnabled` (`self.CapsuleComponent`) "NoCollision")
        (`PrimitiveComponent.SetSimulatePhysics` _mesh true)
        (`SkeletalMeshComponent.PlayAnimation` _mesh null false)
        (set `CharacterMovementComponent.MaxWalkSpeed` 0.0 (`self.CharacterMovement`))
        (`|ExecutionSequence`
          (:`then_0`
            (`KismetSystemLibrary.Delay` 15.0)
            (`self.K2_DestroyActor`))
          (:`then_1`
            (`PrimitiveComponent.SetCastShadow` _mesh_2 false)
            (`SkinnedMeshComponent.SetForcedLOD` _mesh_2 2)
            (`KismetSystemLibrary.K2_ClearTimer` null "ChasePlayer"))
          (:`then_2`
            (bind _returnvalue (`GameplayStatics.GetActorOfClass` "/Game/Blueprints/Zombie/ZombieSpawner_BP.ZombieSpawner_BP_C"))
            (`/Game/Blueprints/Zombie/ZombieSpawner_BP.RebornZombie` _returnvalue)))))
    (elif (`self.IsAttacking`)
      _
      (elif (not (`self.IsRejected`))
        (set `self.IsRejected` true)
        (`|PlayMontage` (`self.Mesh`) (select `int` (`KismetMathLibrary.RandomIntegerInRange` 0 2) :`0` "/Game/ShirtlessZombiesPack/Zombie_Pack/Animations/InPlace/Hits/Zombie_HitReact_Head_Montage.Zombie_HitReact_Head_Montage" :`1` "/Game/ShirtlessZombiesPack/Zombie_Pack/Animations/InPlace/Hits/Zombie_HitReact_LeftArm_Montage.Zombie_HitReact_LeftArm_Montage" :`2` "/Game/ShirtlessZombiesPack/Zombie_Pack/Animations/InPlace/Hits/Zombie_HitReact_RightArm_Montage.Zombie_HitReact_RightArm_Montage" :!type "AnimMontage Object Reference") 1.3
          (:`OnCompleted`
            _)
          (:`OnInterrupted`
            _))
        (set `self.IsRejected` false)))))

(event `attackRangeCheck`
  (bind _returnvalue (`self.K2_GetActorLocation`))
  (bind (_outhit _returnvalue_2) (`KismetSystemLibrary.SphereTraceSingle` _returnvalue (+ _returnvalue (* (`self.GetActorForwardVector`) 160)) 30.0 "TraceTypeQuery3"))
  (if _returnvalue_2
    (if (not (`self.IsAttacking`))
      (set `self.IsAttacking` true)
      (`|PlayMontage` (`self.Mesh`) (select `int` (`KismetMathLibrary.RandomIntegerInRange` 0 3) :`0` "/Game/ShirtlessZombiesPack/Zombie_Pack/Animations/InPlace/Attacks/RM_LeftAttack_Charged_02_Montage.RM_LeftAttack_Charged_02_Montage" :`1` "/Game/ShirtlessZombiesPack/Zombie_Pack/Animations/InPlace/Attacks/RM_RightAttack_Charged_01_Montage.RM_RightAttack_Charged_01_Montage" :`2` "/Game/ShirtlessZombiesPack/Zombie_Pack/Animations/InPlace/Attacks/RM_RightAttack_Charged_02_Montage.RM_RightAttack_Charged_02_Montage" :`3` "/Game/ShirtlessZombiesPack/Zombie_Pack/Animations/InPlace/Attacks/RM_RightAttack_Charged_03_Montage.RM_RightAttack_Charged_03_Montage" :!type "AnimMontage Object Reference") 1.2
        (:`OnCompleted`
          (set `self.IsAttacking` false))))))

(event `HitDamageCheck`
  (bind _mesh (`self.Mesh`))
  (bind (_outhit _returnvalue) (`KismetSystemLibrary.SphereTraceSingle` (`SceneComponent.GetSocketLocation` _mesh (`self.StartSocket`)) (`SceneComponent.GetSocketLocation` _mesh (`self.EndSocket`)) 30.0 "TraceTypeQuery3"))
  (if _returnvalue
    (`/Engine/EditorBlueprintResources/StandardMacros.DoOnce` false :!label _label
      (:`Completed`
        (bind (_bblockinghit _binitialoverlap _time _distance _location _impactpoint _normal _impactnormal _physmat _hitactor) (`GameplayStatics.BreakHitResult` _outhit))
        (`GameplayStatics.ApplyDamage` _hitactor 10.0)
        (`GameplayStatics.SpawnEmitterAtLocation` "/Game/Particles/Effects1/SmokeBuilder/Particles/P_SmokePuff1b.P_SmokePuff1b" _location (`KismetMathLibrary.Conv_VectorToRotator` _normal) (0.1 0.1 0.1))))))

(event `Reset Apply Damege`
  (goto _label :!via `Reset`))

(fn `Init velocity and anim`
  (bind _as_zombie_anim (`self.As Zombie Anim`))
  (switch `int` (`KismetMathLibrary.RandomIntegerInRange` 0 1)
    (:`0`
      (set `/Game/Blueprints/Zombie/Zombie_Anim.MoveAnim` "/Game/ShirtlessZombiesPack/Zombie_Pack/Animations/InPlace/Locomotion/IP_Run_Front.IP_Run_Front" _as_zombie_anim)
      (set `self.Inital velocity` 200.0))
    (:`1`
      (set `/Game/Blueprints/Zombie/Zombie_Anim.MoveAnim` "/Game/ShirtlessZombiesPack/Zombie_Pack/Animations/InPlace/Locomotion/IP_Sprint_Front.IP_Sprint_Front" _as_zombie_anim)
      (set `self.Inital velocity` 480.0)))
  (set `/Game/Blueprints/Zombie/Zombie_Anim.IdleAnim` (select `int` (`KismetMathLibrary.RandomIntegerInRange` 0 2) :`0` "/Game/ShirtlessZombiesPack/Zombie_Pack/Animations/InPlace/Idle/IP_Idle_01.IP_Idle_01" :`1` "/Game/ShirtlessZombiesPack/Zombie_Pack/Animations/InPlace/Idle/IP_Idle_02.IP_Idle_02" :`2` "/Game/ShirtlessZombiesPack/Zombie_Pack/Animations/InPlace/Idle/IP_Idle_08.IP_Idle_08" :!type "AnimSequenceBase Object Reference") _as_zombie_anim)
  (set `/Game/Blueprints/Zombie/Zombie_Anim.Start Position` (`KismetMathLibrary.RandomFloatInRange` 0.0 1.0) (`self.As Zombie Anim`))
  (set `CharacterMovementComponent.MaxWalkSpeed` (`self.Inital velocity`) (`self.CharacterMovement`)))

(fn `RandomZombie`
  (`SkeletalMeshComponent.SetSkeletalMeshAsset` (`self.Mesh`) (select `int` (`KismetMathLibrary.RandomIntegerInRange` 0 4) :`0` "/Game/ShirtlessZombiesPack/UE4/SK_ZombieBB_V1.SK_ZombieBB_V1" :`1` "/Game/ShirtlessZombiesPack/UE4/SK_ZombieBB_V2.SK_ZombieBB_V2" :`2` "/Game/ShirtlessZombiesPack/UE4/SK_ZombieBB_V3.SK_ZombieBB_V3" :`3` "/Game/ShirtlessZombiesPack/UE4/SK_ZombieBB_V4.SK_ZombieBB_V4" :`4` "/Game/ShirtlessZombiesPack/UE4/SK_ZombieBB_V5.SK_ZombieBB_V5" :!type "SkeletalMesh Object Reference")))

(fn `UserConstructionScript`)