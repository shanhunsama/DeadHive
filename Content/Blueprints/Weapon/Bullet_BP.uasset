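; Bullet actor that deals damage on hit, with heavier damage for hits on the "head" bone, and expires shortly after spawning.
; On hit it spawns an attached decal, sound and particle effect, choosing flesh variants for Zombie_BP and concrete variants for everything else.
; It then applies damage to the hit actor, pushes physics-simulating components with a velocity-scaled impulse, and destroys itself.
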(event `self.ReceiveBeginPlay`
  (`self.SetLifeSpan` 1.0))

(event `self.ReceiveHit`
  (params (MyComp :type "PrimitiveComponent Object Reference") (Other :type "Actor Object Reference") (OtherComp :type "PrimitiveComponent Object Reference") (bSelfMoved :type Boolean) (HitLocation :type "Vector Structure") (HitNormal :type "Vector Structure") (NormalImpulse :type "Vector Structure") (Hit :type "HitResult Structure (by ref)"))
  (bind (_bblockinghit _binitialoverlap _time _distance _location _impactpoint _normal _impactnormal _physmat _hitactor _hitcomponent _hitbonename) (`GameplayStatics.BreakHitResult` Hit))
  (bind (_aszombie_bp _bsuccess) (cast `/Game/Blueprints/Zombie/Zombie_BP` Other :!pure true))
  (bind _returnvalue (`KismetMathLibrary.Conv_VectorToRotator` _impactnormal))
  (bind _returnvalue_2 (`GameplayStatics.SpawnDecalAttached` (select `bool` _bsuccess :`false` "/Game/Particles/Bullet_Impact_Decal.Bullet_Impact_Decal" :`true` "/Game/Particles/blood_Mat.blood_Mat" :!type "MaterialInterface Object Reference") (7.0 7.0 7.0) OtherComp _hitbonename _impactpoint _returnvalue "KeepWorldPosition" 20.0))
  (`/Engine/EditorBlueprintResources/StandardMacros.IsValid` _returnvalue_2
    (:`Is Valid`
      (`DecalComponent.SetFadeScreenSize` _returnvalue_2 0.0))
    (:`Is Not Valid`
      _))
  (`GameplayStatics.PlaySoundAtLocation` (select `bool` _bsuccess :`false` "/Game/Sounds/BulletImpact/Concrete/bullet_impact_concrete_brick_08_Cue.bullet_impact_concrete_brick_08_Cue" :`true` "/Game/Sounds/BulletImpact/Body/bullet_impact_body_flesh_01_Cue.bullet_impact_body_flesh_01_Cue" :!type "SoundBase Object Reference") _impactpoint (struct) 1.0 1.0 0.0 null null null null)
  (`GameplayStatics.SpawnEmitterAtLocation` (select `bool` _bsuccess :`false` "/Game/Particles/bulletvfx/Particles/VFX_Impact_Concrete.VFX_Impact_Concrete" :`true` "/Game/Particles/bulletvfx/Particles/VFX_Impact_Flesh.VFX_Impact_Flesh" :!type "ParticleSystem Object Reference") _impactpoint _returnvalue)
  (`self.TakeDamageOnZombie` Hit)
  (`|ExecutionSequence`
    (:`then_0`
      (`/Engine/EditorBlueprintResources/StandardMacros.IsValid` OtherComp
        (:`Is Valid`
          (if (`SceneComponent.IsSimulatingPhysics` OtherComp "None")
            (`PrimitiveComponent.AddImpulse` OtherComp (* (`self.GetVelocity`) 25.0) _hitbonename false)))))
    (:`then_1`
      (`self.K2_DestroyActor`))))

(fn `TakeDamageOnZombie`
  (params (Hit :type "HitResult Structure"))
  (bind (_bblockinghit _binitialoverlap _time _distance _location _impactpoint _normal _impactnormal _physmat _hitactor _hitcomponent _hitbonename) (`GameplayStatics.BreakHitResult` Hit))
  (if (== _hitbonename "head")
    (`GameplayStatics.ApplyDamage` _hitactor 100.0)
    (else
      (`GameplayStatics.ApplyDamage` _hitactor 40.0))))

(fn `UserConstructionScript`)