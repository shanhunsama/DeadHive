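; Player rifle weapon actor handling automatic fire, ammo and reloading, with arm and gun montages chosen by aim and magazine state.
; A looping timer spawns Bullet_BP at the muzzle socket, straight when aiming or within a random cone otherwise.
; Each shot triggers timeline-driven recoil through controller yaw and pitch input.
; Reload empties the magazine count until the gun montage completes, then calculates the refill from reserve ammo.
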(event EventBeginPlay
  (bind _asplayer_bp (Utilities|Casting|CastToPlayer_BP (Game|Player|GetPlayerPawn 0)))
  (Variables|Default|SetAs%20Player%20BP _asplayer_bp)
  (Variables|Default|SetCur%20Bullets%20Num (Variables|Default|GetMaxCapacityBulletNum))
  (Variables|Default|SetTotalBulletNum 300))

(event Collision|EventActorBeginOverlap
  (params (OtherActor :type Actor%20Object%20Reference)))

(event EventTick
  (params (DeltaSeconds :type Float%20%28single-precision%29)))

(event Custom|StartShoot
  (Utilities|Time|SetTimerbyFunctionName 0 "OnShooting" 0.12 true)
  (CallFunction|OnShooting))

(event Custom|StartReload
  (if (> (Variables|Default|GetTotalBulletNum) 0)
    (if (not (== (Variables|Default|GetCur%20Bullets%20Num) (Variables|Default|GetMaxCapacityBulletNum)))
      (if (not (Variables|Default|GetIsReloading))
        (Variables|Default|SetIsReloading true)
        (Variables|Default|SetBulletTemp (Variables|Default|GetCur%20Bullets%20Num))
        (Variables|Default|SetCur%20Bullets%20Num 0)
        (Animation|Montage|PlayMontage (Variables|/Script/Engine.Character|GetMesh (Variables|Default|GetAs%20Player%20BP)) (select (> (Variables|Default|GetBulletTemp) 0) "/Game/FPS_Assault_Pack/Animations/RU74/A_Arms_RU74_Reload_Montage.A_Arms_RU74_Reload_Montage" "/Game/FPS_Assault_Pack/Animations/RU74/A_Arms_RU74_Reload_Empty_Montage.A_Arms_RU74_Reload_Empty_Montage")
          (:then
            (Animation|Montage|PlayMontage (Variables|Default|GetSkeletalMesh) (select (> (Variables|Default|GetBulletTemp) 0) "/Game/FPS_Assault_Pack/Animations/RU74/A_RU74_Reload_Montage.A_RU74_Reload_Montage" "/Game/FPS_Assault_Pack/Animations/RU74/A_RU74_Reload_Empty_Montage.A_RU74_Reload_Empty_Montage")
              (:OnCompleted
                (Variables|Default|SetIsReloading false)
                (CallFunction|CaculateLostBullets)
                (Variables|Default|SetCur%20Bullets%20Num (Variables|Default|GetBulletTemp))))))))))

(event Custom|OnShooting
  (bind (_return_value_location _returnvalue) (CallFunction|BulletsLocandRot))
  (bind _as_player_bp (Variables|Default|GetAs%20Player%20BP))
  (bind _as_player_anim (Variables|/Game/Blueprints/Character/Player_BP.Player_BP_C|GetAs%20Player%20Anim _as_player_bp))
  (if (<= (Variables|Default|GetCur%20Bullets%20Num) 0)
    (Audio|PlaySound2D "/Game/Sounds/Weapon/AK74/gun_rifle_dry_fire_04_Cue.gun_rifle_dry_fire_04_Cue" 1.0 1.0 0.0 0 0)
    (Utilities|Time|ClearTimerbyFunctionName 0 "OnShooting")
    (else
      (Animation|Montage|MontagePlay _as_player_anim (select (Variables|/Game/Blueprints/Character/Player_Anim.Player_Anim_C|GetisAimming _as_player_anim) "/Game/FPS_Assault_Pack/Animations/RU74/A_Arms_RU74_Isight_Shoot01_Montage.A_Arms_RU74_Isight_Shoot01_Montage" "/Game/FPS_Assault_Pack/Animations/RU74/A_Arms_RU74_Shoot02_Montage.A_Arms_RU74_Shoot02_Montage") 1.2 "MontageLength" 0.0 true)
      (Animation|Montage|MontagePlay (Components|SkeletalMesh|GetAnimInstance (Variables|Default|GetSkeletalMesh)) "/Game/FPS_Assault_Pack/Animations/RU74/A_RU74_Shoot01_Montage.A_RU74_Shoot01_Montage" 2.5 "MontageLength" 0.0 true)
      (Game|SpawnActorfromClass "/Game/Blueprints/Weapon/Bullet_BP.Bullet_BP_C" (Math|Transform|MakeTransform _return_value_location _returnvalue "0.100000,0.100000,0.100000") "AlwaysSpawn" "MultiplyWithRoot" 0 0)
      (Variables|Default|SetCur%20Bullets%20Num (- (Variables|Default|GetCur%20Bullets%20Num) 1))
      (CallFunction|RecoilCaculate))))

(event Custom|Stop%20Shoot
  (Utilities|Time|ClearTimerbyFunctionName 0 "OnShooting"))

(event Custom|Recoil%20caculate
  (bind _returnvalue (Game|Player|GetPlayerPawn 0))
  (bind _新建轨道_0 (Timeline|时间轴 PlayFromStart)
    (:Update
      (Pawn|Input|AddControllerYawInput _returnvalue (Math|Random|RandomFloatinRange -0.1 0.1))
      (Pawn|Input|AddControllerPitchInput _returnvalue (Math|Float|Lerp 0.0 -0.1 _新建轨道_0)))))

(event Input|KeyboardEvents|DebugKeyP
  (params (Key :type Key%20Structure :default "None") (ActionValue :type Input%20Action%20Value%20Structure)))

(fn ConstructionScript)

(fn CaculateLostBullets
  (if (> (- (Variables|Default|GetTotalBulletNum) (- (Variables|Default|GetMaxCapacityBulletNum) (Variables|Default|GetBulletTemp))) 0)
    (Variables|Default|SetTotalBulletNum (- (Variables|Default|GetTotalBulletNum) (- (Variables|Default|GetMaxCapacityBulletNum) (Variables|Default|GetBulletTemp))))
    (Variables|Default|SetBulletTemp (Variables|Default|GetMaxCapacityBulletNum))
    (else
      (Variables|Default|SetCur%20Bullets%20Num (+ (Variables|Default|GetBulletTemp) (Variables|Default|GetTotalBulletNum)))
      (Variables|Default|SetTotalBulletNum 0)))
  (return))

(fn BulletsLocandRot
  (bind _skeletalmesh (Variables|Default|GetSkeletalMesh))
  (bind _returnvalue (Transformation|GetSocketTransform _skeletalmesh "b_Muzzle插槽" "RTS_World"))
  (return (.location _returnvalue) (select (Variables|/Game/Blueprints/Character/Player_Anim.Player_Anim_C|GetisAimming (Variables|/Game/Blueprints/Character/Player_BP.Player_BP_C|GetAs%20Player%20Anim (Variables|Default|GetAs%20Player%20BP))) (.rotation _returnvalue) (Math|Conversions|RotationFromXVector (Math|Random|RandomUnitVectorinConeinDegrees (Math|Rotator|GetRotationXVector (.rotation _returnvalue)) 5.0)))))