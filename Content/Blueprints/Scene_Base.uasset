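; Scene_Base sets up the main menu scene when play begins.
; It creates and shows the MainMenu_UWG widget, then switches the player's view to one of two targets picked at random.
; It focuses Game-and-UI input on the menu with the mouse locked, then starts the background music as a 2D sound, keeping references to both widget and music.
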(event `self.ReceiveBeginPlay`
  (bind _returnvalue (`GameplayStatics.GetPlayerController` 0))
  (bind _returnvalue_2 (`|CreateWidget` "/Game/UI/MainMenu_UWG.MainMenu_UWG_C"))
  (bind _output_get (set `self.MainMenu` _returnvalue_2))
  (`UserWidget.AddToViewport` _output_get 0)
  (`PlayerController.SetViewTargetWithBlend` _returnvalue (select `int` (`KismetMathLibrary.RandomIntegerInRange` 0 1) :`0` "" :`1` "") 0.0 "VTBlend_Linear" 0.0 false)
  (`WidgetBlueprintLibrary.SetInputMode_GameAndUIEx` _returnvalue _output_get "LockAlways" false)
  (bind _returnvalue_3 (`GameplayStatics.SpawnSound2D` "/Game/UI/Sounds/WAV_Survival2_Departure_Strings.WAV_Survival2_Departure_Strings" 1.0 1.0 0.0 null))
  (set `self.BGM` _returnvalue_3))

(fn `UserConstructionScript`)